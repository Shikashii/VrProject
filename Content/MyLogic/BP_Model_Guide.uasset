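; BP_Model_Guide is a step-by-step visual guide that reveals and highlights a model's parts in construction order.
; Index change events and BeginPlay run a shared pass matching PartInfo construction indices to static mesh components tagged with part names.
; The current mesh in the group is unhidden and tinted green, while the preceding mesh and all meshes of the preceding step are set to Mat0.
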(event `IndexInGroupChanged`
  (params (NewIndexInGroup :type Integer))
  (bind (_partinfo_partreferens _partinfo_partname _partinfo_partimage _partinfo_isneedsupports _partinfo_partmass _partinfo_partprinttime _partinfo_partamountneeded _partinfo_partamountchosen _partinfo_partchosensupports _partinfo_constructionindex) (break `/Game/MyLogic/S_PartInfo` (`self.PartInfo`)))
  (set `self.IndexInGroupMG` NewIndexInGroup)
  (for (_array_element _array_index) _partinfo_constructionindex :!label _label
    (if (== _array_element (`self.CurrentIndexMG`))
      (bind _returnvalue (`self.GetComponentsByTag` "/Script/Engine.StaticMeshComponent" (`KismetStringLibrary.Conv_StringToName` (`|GetArrayItem` _partinfo_partname _array_index))))
      (bind _output (`|GetArrayItem` _returnvalue (`self.IndexInGroupMG`)))
      (`SceneComponent.SetHiddenInGame` _output false false)
      (`PrimitiveComponent.SetMaterial` _output 0 "/AnimationSharing/AnimSharingGreen.AnimSharingGreen")
      (if (> (`self.IndexInGroupMG`) 0)
        (`PrimitiveComponent.SetMaterial` (`|GetArrayItem` _returnvalue (- (`self.IndexInGroupMG`) 1)) 0 "/Game/MyLogic/Parts/mat0.mat0"))
      (elif (== _array_element (- (`self.CurrentIndexMG`) 1))
        (for _array_element_2 _returnvalue
          (`PrimitiveComponent.SetMaterial` _array_element_2 0 "/Game/MyLogic/Parts/mat0.mat0"))))))

(event `IndexChanged`
  (params (NewIndex :type Integer))
  (set `self.CurrentIndexMG` NewIndex)
  (set `self.IndexInGroupMG` 0)
  (goto _label))

(event `self.ReceiveBeginPlay`
  (goto _label))

(fn `UserConstructionScript`)