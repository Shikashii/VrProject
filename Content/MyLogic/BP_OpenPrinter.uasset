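; Actor that floats a printer prompt widget in front of the camera and opens the printer menu when clicked.
; Tick and OpenPrinterWidget share one update that places the actor just ahead of CamRef and matches the SpringArm to the camera's rotation.
; ClickOnPrinter, if the widget is visible, shows the first BP_PrinterPlaceHolder's PrinterMenu, hides this actor's components and calls YouNeedToPrint on the first WB_Menu.
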(event `self.ReceiveTick`
  (params (DeltaSeconds :type "Float (single-precision)"))
  (`self.K2_SetActorLocation` (+ (`SceneComponent.K2_GetComponentLocation` (stale `OpenPrinterWidget` CamRef)) (* (`SceneComponent.GetForwardVector` (stale `OpenPrinterWidget` CamRef)) 100.0)) :!label _label)
  (`SceneComponent.K2_SetWorldRotation` (`self.SpringArm`) (`SceneComponent.K2_GetComponentRotation` (stale `OpenPrinterWidget` CamRef)) false false))

(event `OpenPrinterWidget`
  (params (CamRef :type "CameraComponent Object Reference"))
  (goto _label))

(event `ClickOnPrinter`
  (if (`SceneComponent.IsVisible` (`self.Widget`))
    (bind _outactors (`GameplayStatics.GetAllActorsOfClass` "/Game/MyLogic/BP_PrinterPlaceHolder.BP_PrinterPlaceHolder_C"))
    (`SceneComponent.SetVisibility` (`/Game/MyLogic/BP_PrinterPlaceHolder.PrinterMenu` (`|GetArrayItem` _outactors)) true false)
    (`SceneComponent.SetVisibility` (`self.DefaultSceneRoot`) false true)
    (bind _foundwidgets (`WidgetBlueprintLibrary.GetAllWidgetsOfClass` "/Game/MyLogic/Menu/WB_Menu.WB_Menu_C" false))
    (`/Game/MyLogic/Menu/WB_Menu.YouNeedToPrint` (`|GetArrayItem` _foundwidgets))))

(fn `UserConstructionScript`)