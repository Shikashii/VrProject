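; BP_TablePlaceholder is a proximity trigger that advances the menu's quest to a crafting step when the VR player comes near it.
; Each Tick until it fires, it finds the first VRPawn and measures the distance from that pawn's camera to its own root.
; Once within range, it sets IsQuestChanged so it runs only once, then calls YouNeedToCraft on the first WB_Menu widget found.
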(event `self.ReceiveTick`
  (params (DeltaSeconds :type "Float (single-precision)"))
  (if (not (`self.IsQuestChanged`))
    (bind _outactors (`GameplayStatics.GetAllActorsOfClass` "/Game/VRTemplate/Blueprints/VRPawn.VRPawn_C"))
    (if (< (`KismetMathLibrary.VSize` (- (`SceneComponent.K2_GetComponentLocation` (`/Game/VRTemplate/Blueprints/VRPawn.Camera` (`|GetArrayItem` _outactors))) (`SceneComponent.K2_GetComponentLocation` (`self.DefaultSceneRoot`)))) 350.0)
      (set `self.IsQuestChanged` true)
      (bind _foundwidgets (`WidgetBlueprintLibrary.GetAllWidgetsOfClass` "/Game/MyLogic/Menu/WB_Menu.WB_Menu_C" false))
      (`/Game/MyLogic/Menu/WB_Menu.YouNeedToCraft` (`|GetArrayItem` _foundwidgets)))))

(fn `UserConstructionScript`)