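; BP_PrinterPlaceHolder is a printer stand-in that opens a printer menu when a nearby VR player points at it.
; Tick checks whether the first VRPawn is within a fixed range and hides the menu actor when it is not.
; When the pawn's ViewPointer overlaps the Box in range, it spawns BP_OpenPrinter at the camera or re-shows the existing one, then calls OpenPrinterWidget.
; Ending the overlap hides that actor.
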(event `self.ReceiveTick`
  (params (DeltaSeconds :type "Float (single-precision)"))
  (bind _openref (`self.OpenRef`))
  (bind _outactors (`GameplayStatics.GetAllActorsOfClass` "/Game/VRTemplate/Blueprints/VRPawn.VRPawn_C"))
  (if (< (`KismetMathLibrary.VSize` (- (`self.K2_GetActorLocation` (`|GetArrayItem` _outactors)) (`self.K2_GetActorLocation`))) 350.0)
    (set `self.IsPlayerNearby` true)
    (else
      (set `self.IsPlayerNearby` false)
      (`/Engine/EditorBlueprintResources/StandardMacros.IsValid` _openref
        (:`Is Valid`
          (`SceneComponent.SetVisibility` (`/Game/MyLogic/BP_OpenPrinter.DefaultSceneRoot` _openref) false true))))))

(event `self.Box.OnComponentBeginOverlap`
  (params (OverlappedComponent :type "PrimitiveComponent Object Reference") (OtherActor :type "Actor Object Reference") (OtherComp :type "PrimitiveComponent Object Reference") (OtherBodyIndex :type Integer) (bFromSweep :type Boolean) (SweepResult :type "HitResult Structure (by ref)"))
  (bind _openref (`self.OpenRef`))
  (if (== (`/Game/VRTemplate/Blueprints/VRPawn.ViewPointer` (`|GetArrayItem` (stale `self.ReceiveTick` _outactors))) OtherComp)
    (if (`self.IsPlayerNearby`)
      (`/Engine/EditorBlueprintResources/StandardMacros.IsValid` _openref
        (:`Is Valid`
          (`SceneComponent.SetVisibility` (`/Game/MyLogic/BP_OpenPrinter.DefaultSceneRoot` _openref) true true))
        (:`Is Not Valid`
          (bind _outactors (`GameplayStatics.GetAllActorsOfClass` "/Game/VRTemplate/Blueprints/VRPawn.VRPawn_C"))
          (bind _camera (`/Game/VRTemplate/Blueprints/VRPawn.Camera` (`|GetArrayItem` _outactors)))
          (bind _returnvalue (`|SpawnActorFromClass` "/Game/MyLogic/BP_OpenPrinter.BP_OpenPrinter_C" (`KismetMathLibrary.MakeTransform` (`SceneComponent.K2_GetComponentLocation` _camera) (`SceneComponent.K2_GetComponentRotation` _camera)) "Undefined" "OverrideRootScale" null null))
          (bind _output_get (set `self.OpenRef` _returnvalue))
          (`self.SetActorHiddenInGame` _output_get false)))
      (`/Game/MyLogic/BP_OpenPrinter.OpenPrinterWidget` (`self.OpenRef`) _camera))))

(event `self.Box.OnComponentEndOverlap`
  (params (OverlappedComponent :type "PrimitiveComponent Object Reference") (OtherActor :type "Actor Object Reference") (OtherComp :type "PrimitiveComponent Object Reference") (OtherBodyIndex :type Integer))
  (bind _openref (`self.OpenRef`))
  (if (== (`/Game/VRTemplate/Blueprints/VRPawn.ViewPointer` (`|GetArrayItem` (stale `self.ReceiveTick` _outactors))) OtherComp)
    (`/Engine/EditorBlueprintResources/StandardMacros.IsValid` _openref
      (:`Is Valid`
        (`SceneComponent.SetVisibility` (`/Game/MyLogic/BP_OpenPrinter.DefaultSceneRoot` _openref) false true)))))

(event `ClosePrinterMenu`
  (`SceneComponent.SetVisibility` (`self.PrinterMenu`) false true))

(fn `UserConstructionScript`)