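; BP_Menu is a world-space menu actor that is placed in front of the player camera and hides when the player looks away.
; InventoryOpen moves it 200 units along the camera's forward vector, aligns its SpringArm to the camera rotation and stores that direction.
; Each Tick compares the stored direction with the current camera forward, hiding the root and its children beyond 45 degrees; this graph never re-shows them.
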(event `self.ReceiveTick`
  (params (DeltaSeconds :type "Float (single-precision)"))
  (if (> (`KismetMathLibrary.DegAcos` (`KismetMathLibrary.Dot_VectorVector` (`self.MenuDirection`) (`self.GetActorForwardVector` (`GameplayStatics.GetPlayerCameraManager` 0)))) 45.0)
    (`SceneComponent.SetVisibility` (`self.DefaultSceneRoot`) false true)))

(event `InventoryOpen`
  (bind _returnvalue (`GameplayStatics.GetPlayerCameraManager` 0))
  (bind _returnvalue_2 (`self.GetActorForwardVector` _returnvalue))
  (bind (_returnvalue_location _returnvalue_rotation) (`KismetMathLibrary.BreakTransform` (`self.GetTransform` _returnvalue)))
  (`self.K2_SetActorLocation` (+ _returnvalue_location (* _returnvalue_2 200.0)))
  (`SceneComponent.K2_SetWorldRotation` (`self.SpringArm`) _returnvalue_rotation false false)
  (set `self.MenuDirection` _returnvalue_2))

(fn `UserConstructionScript`)