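; BP_Door is a door actor that swings open on a timeline and carries a door prompt widget.
; YouNeedToDeleteSups shows the widget with a "remove supports" text in Russian and reveals its delete button, taking the second WB_Door instance found.
; The 1stDoorOpen and 2ndDoorOpen events each pass a DoOnce into the shared timeline, whose update rotates the door and hides the widget.
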(event `YouNeedToDeleteSups`
  (bind _foundwidgets (`WidgetBlueprintLibrary.GetAllWidgetsOfClass` "/Game/MyLogic/WB_Door.WB_Door_C" false))
  (bind _output (`|GetArrayItem` _foundwidgets 1))
  (`Widget.SetVisibility` (`/Game/MyLogic/WB_Door.DeleteSupButton` _output) "Visible")
  (`TextBlock.SetText` (`/Game/MyLogic/WB_Door.DoorText` _output) "Убрать поддержки")
  (`SceneComponent.SetVisibility` (`self.DoorWidget`) true false))

(event `2ndDoorOpen`
  (`/Engine/EditorBlueprintResources/StandardMacros.DoOnce` false
    (:`Completed`
      (bind (_direction _newtrack_0) (`Timeline|Timeline_0` :!via `PlayFromStart` :!label _label)
        (:`Update`
          (`SceneComponent.K2_SetRelativeRotation` (`self.Door`) (`KismetMathLibrary.RLerp` (struct) (struct :`Yaw` 100.0) _newtrack_0) false false)
          (`SceneComponent.SetVisibility` (`self.DoorWidget`) false false))))))

(event `1stDoorOpen`
  (`/Engine/EditorBlueprintResources/StandardMacros.DoOnce` false
    (:`Completed`
      (goto _label :!via `PlayFromStart`))))

(fn `UserConstructionScript`)